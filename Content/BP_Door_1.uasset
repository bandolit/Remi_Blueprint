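; BP_Door_1 is a double door that swings open and closed when interacted with.
; The Interaction event runs only while the Open flag is true, then a FlipFlop alternates between playing and reversing the Test timeline.
; The timeline track, scaled by RotationAngle, sets the relative yaw of the two door meshes in opposite directions.
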(event `/Game/Blueprints/Implemented/BPI_Interaction.Interaction`
  (if (`self.open`)
    (`/Engine/EditorBlueprintResources/StandardMacros.FlipFlop`
      (:`A`
        (bind (_direction _newtrack_0) (`Timeline|Test` :!label _label)
          (:`Update`
            (bind _returnvalue (* _newtrack_0 (`self.rotation angle`)))
            (`SceneComponent.K2_SetRelativeRotation` (`self.Door_3_StaticMeshComponent0`) (`KismetMathLibrary.MakeRotator` 0.0 0.0 (* _returnvalue -1.0)) false false)
            (`SceneComponent.K2_SetRelativeRotation` (`self.Door_4_StaticMeshComponent0`) (`KismetMathLibrary.MakeRotator` 0.0 0.0 _returnvalue) false false))))
      (:`B`
        (goto _label :!via `Reverse`)))))

(fn `UserConstructionScript`)